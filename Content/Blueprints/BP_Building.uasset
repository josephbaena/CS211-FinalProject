(event `self.ReceiveBeginPlay`)

(event `self.ReceiveActorBeginOverlap`
  (params (OtherActor :type "Actor Object Reference")))

(event `self.ReceiveTick`
  (params (DeltaSeconds :type "Float (single-precision)")))

(fn `Build`
  (params (x :type Integer) (y :type Integer) (z :type Integer))
  (bind _space (`self.Space`))
  (bind _length (`self.Length`))
  (set `self.Y` y)
  (set `self.X` x)
  (set `self.Z` z)
  (for _index (range (+ (`self.X`) 1))
    (for _index_2 (range (+ (`self.Y`) 1))
      (for _index_3 (range (+ (`self.Z`) 1))
        (bind _returnvalue (`AddComponent|StaticMeshComponent_46673`))
        (`SceneComponent.K2_AttachTo` _returnvalue (`self.Tile`) "None" "KeepRelativeOffset" false)
        ;[1 1 1] Set Properties
        (`SceneComponent.K2_SetRelativeLocation` _returnvalue (`KismetMathLibrary.MakeVector` (+ (* _index_2 _space) (* _index_2 _length) 0.0) (+ (* _index _space) (* _index _length) 0.0) (+ (* _index_3 _space) (* _index_3 _length) 0.0)) false)
        (`SceneComponent.SetRelativeScale3D` (`KismetMathLibrary.Conv_DoubleToVector` (`self.Scale`)))))))

(fn `UserConstructionScript`)