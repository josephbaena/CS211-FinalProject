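; BP_PointSystem is an Actor that keeps a replicated, time-based score and shows it on a label.
; On Tick, only the authority runs a half-second Delay, which ignores re-triggers while pending, so UpdateScore adds one point roughly every half second.
; The Score RepNotify writes the new value to ScoreLabel whenever it changes.
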(event `self.ReceiveBeginPlay`)

(event `self.ReceiveActorBeginOverlap`
  (params (OtherActor :type "Actor Object Reference")))

(event `self.ReceiveTick`
  (params (DeltaSeconds :type "Float (single-precision)"))
  (`/Engine/EditorBlueprintResources/ActorMacros.Switch Has Authority`
    (:`Authority`
      (`KismetSystemLibrary.Delay` 0.5)
      (`self.Update_Score`))))

(fn `OnRep_Score`
  (`TextRenderComponent.SetText` (`self.ScoreLabel`) (`KismetStringLibrary.Conv_IntToString` (`self.Score`))))

(fn `Update_Score`
  (set `self.Score` (+ (`self.Score`) 1)))

(fn `UserConstructionScript`)