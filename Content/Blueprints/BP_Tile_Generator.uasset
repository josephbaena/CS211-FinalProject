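; BP_Tile_Generator is a procedural actor that builds a grid of static mesh tiles in its construction script.
; Nested loops over X and Y add a mesh component per cell, attach it to Tile and position it by tile length and spacing.
; Each tile gets a random height and yaw scaled by variation variables, using unseeded randomness, while the event graph holds no active logic.
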(event `self.ReceiveBeginPlay`)

(event `self.ReceiveActorBeginOverlap`
  (params (OtherActor :type "Actor Object Reference")))

(event `self.ReceiveTick`
  (params (DeltaSeconds :type "Float (single-precision)")))

(fn `UserConstructionScript`
  (bind _space (`self.Space`))
  (bind _length (`self.Length`))
  (for _index (range (+ (`self.X`) 1))
    (for _index_2 (range (+ (`self.Y`) 1))
      (bind _returnvalue (`AddComponent|Static Mesh Component_5740`))
      (`SceneComponent.K2_AttachTo` _returnvalue (`self.Tile`) "None" "KeepRelativeOffset" true)
      ;[1 1 1] Set Properties
      (`SceneComponent.K2_SetRelativeLocation` _returnvalue (`KismetMathLibrary.MakeVector` (+ (* _index_2 _space) (* _index_2 _length) 0.0) (+ (* _index _length) (* _index _space)) (* (`self.Height Variation`) (`KismetMathLibrary.RandomFloat`))) false)
      (`SceneComponent.K2_SetRelativeRotation` _returnvalue (`KismetMathLibrary.MakeRot` 0.0 (* (`KismetMathLibrary.RandomFloat`) (`self.Rotation Variation`))) false))))