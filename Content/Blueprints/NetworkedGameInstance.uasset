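; Game instance Blueprint that handles hosting, joining and leaving multiplayer sessions, with a configurable LAN option.
; Hosting creates a session, then opens the game level as a listen server.
; Joining searches for sessions and joins the first result, writing searching or not-found status to every BP_SessionJoiner actor's text.
; Leaving destroys the session and opens the lobby level, also with the listen option.
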(event `HostGameEvent`
  (`CreateSessionCallbackProxy.CreateSession` (`GameplayStatics.GetPlayerController` 0) 4 (`self.UseLan?`)
    (:`OnSuccess`
      (`GameplayStatics.OpenLevel` (`self.LevelString`) true "listen"))))

(event `JoinGame`
  (bind _results (`FindSessionsCallbackProxy.FindSessions` (`GameplayStatics.GetPlayerController` 0) 4 (`self.UseLan?`))
    (:`then`
      (bind _outactors (`GameplayStatics.GetAllActorsOfClass` "/Game/Blueprints/BP_SessionJoiner.BP_SessionJoiner_C"))
      (for _array_element _outactors
        (`TextRenderComponent.SetText` (`/Game/Blueprints/BP_SessionJoiner.StatusText` _array_element) "Searching for Sessions...")))
    (:`OnSuccess`
      (if (== (`KismetArrayLibrary.Array_Length` _results) 0)
        (bind _outactors_2 (`GameplayStatics.GetAllActorsOfClass` "/Game/Blueprints/BP_SessionJoiner.BP_SessionJoiner_C"))
        (for _array_element_2 _outactors_2
          (`TextRenderComponent.SetText` (`/Game/Blueprints/BP_SessionJoiner.StatusText` _array_element_2) "No session found!"))
        (else
          (`JoinSessionCallbackProxy.JoinSession` (`GameplayStatics.GetPlayerController` 0) (`KismetArrayLibrary.Array_Get` _results)))))))

(event `LeaveGame`
  (`DestroySessionCallbackProxy.DestroySession` (`GameplayStatics.GetPlayerController` 0)
    (:`OnSuccess`
      (`GameplayStatics.OpenLevel` (`self.LobbyLevelString`) true "listen"))))